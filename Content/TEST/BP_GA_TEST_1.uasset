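; BP_GA_TEST_1 is a test Gameplay Ability that plays a montage and applies a test gameplay effect to its owner.
; Activation starts the montage task with a TEST event tag, applies BP_GE_TEST right away, and ends the ability when the montage completes, blends out, is interrupted or is cancelled.
; Debug prints mark activation and end; cooldown commit, effect-container and SetByCaller damage nodes sit unconnected.
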(event Ability|EventOnEndAbility
  (params (bWasCancelled :type Boolean))
  (if bWasCancelled
    (Development|PrintString "GA TEST 1 Cancelled" true true "(R=1.000000,G=0.000000,B=0.000000,A=1.000000)" 1e+01)
    (else
      (Development|PrintString "GA TEST 1 End" true true "(R=0.000000,G=0.660000,B=1.000000,A=1.000000)" 1e+01))))

(event Ability|EventActivateAbility
  (Development|PrintString "GA TEST 1" true true "(R=0.000000,G=0.660000,B=1.000000,A=1.000000)" 1e+01)
  (|PlayMontageandWaitEventProxy "None" 0 "(GameplayTags=((TagName=\"TEST\")))" 1.0 "None" true 1.0
    (:then
      (Ability|ApplyGameplayEffectToOwner "/Game/TEST/BP_GE_TEST.BP_GE_TEST_C"))
    (:OnMontageCompletedDelegate
      (Ability|EndAbility :!label _label))
    (:OnMontageBlendOutDelegate
      (goto _label))
    (:OnMontageInterruptedDelegate
      (goto _label))
    (:OnMontageCancelledDelegate
      (goto _label))))