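; Base weapon Blueprint that turns trigger box overlaps during attacks into gameplay events.
; BeginWeaponAttack stores a tag and enables query-only collision; EndWeaponAttack, also run at BeginPlay, clears both.
; The CheckValidTarget macro rejects instigator, owner and self, using a DoOnce re-armed after a retriggerable delay on end overlap to limit repeat hits.
; Valid hits send the tagged event to the instigator with the target in the payload; ResetEquipMesh is an empty hook.
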(event OnComponentBeginOverlap(TriggerBoxComponent)
  (params (OverlappedComponent :type Primitive%20Component%20Object%20Reference) (OtherActor :type Actor%20Object%20Reference) (OtherComp :type Primitive%20Component%20Object%20Reference) (OtherBodyIndex :type Integer) (bFromSweep :type Boolean) (SweepResult :type Hit%20Result%20Structure%20%28by%20ref%29))
  (bind _returnvalue (Game|GetInstigator))
  (bind _tag (Variables|Default|GetTag))
  (bind _targetactor (Utilities|CheckValidTarget OtherActor 0.2)
    (:true
      (Ability|SendGameplayEventtoActor _returnvalue _tag (Utilities|Struct|MakeGameplayEventData _tag _returnvalue _targetactor)))))

(event OnComponentEndOverlap(TriggerBoxComponent)
  (params (OverlappedComponent :type Primitive%20Component%20Object%20Reference) (OtherActor :type Actor%20Object%20Reference) (OtherComp :type Primitive%20Component%20Object%20Reference) (OtherBodyIndex :type Integer))
  (bind _returnvalue (Game|GetInstigator))
  (bind _tag (Variables|Default|GetTag))
  (Utilities|CheckValidTarget (stale OnComponentBeginOverlap(TriggerBoxComponent) OtherActor) 0.2) ; enters at Reset
)

(event EventResetEquipMesh)

(event EventBeginWeaponAttack
  (params (Tag :type Gameplay%20Tag%20Structure%20%28by%20ref%29))
  (Variables|Default|SetTag Tag)
  (Variables|Default|SetIsAttacking true)
  (Variables|/Script/Engine.PrimitiveComponent|SetbGenerateOverlapEvents (Variables|Default|GetTriggerBoxComponent) true)
  (Collision|SetCollisionEnabled (Variables|Default|GetTriggerBoxComponent) "QueryOnly"))

(event EventEndWeaponAttack
  (Variables|Default|SetTag "")
  (Variables|Default|SetIsAttacking false)
  (Variables|/Script/Engine.PrimitiveComponent|SetbGenerateOverlapEvents (Variables|Default|GetTriggerBoxComponent) false)
  (Collision|SetCollisionEnabled (Variables|Default|GetTriggerBoxComponent) "NoCollision"))

(event EventBeginPlay
  (Class|SRWeaponBase|EndWeaponAttack)
  (Class|SREquipmentBase|ResetEquipMesh))

(fn ConstructionScript)