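; BP_SkillActor_Base is a base actor for skills, supplying a shared way to apply gameplay effects to a target.
; MakeAndApplyEffect checks the target is valid, then builds an effect container spec from the instigator, Container, EventData and Level.
; It wraps the target in a synthetic hit result at the target's location, adds it to the spec and applies it.
; Event graph and construction script are empty.
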(event EventBeginPlay)

(event Collision|EventActorBeginOverlap
  (params (OtherActor :type Actor%20Object%20Reference)))

(event EventTick
  (params (DeltaSeconds :type Float%20%28single-precision%29)))

(fn ConstructionScript)

(fn MakeandApplyEffect
  (params (Target :type Actor%20Object%20Reference))
  (bind _output_get (LocalVariables|Set_Target Target))
  (Utilities|IsValid _output_get
    (:Is%20Valid
      (bind _returnvalue (Class|FuncLibAbility|MakeEffectContainerExtra (Game|GetInstigator) (Variables|Default|GetContainer) (Variables|Default|GetEventData) (Variables|Default|GetLevel)))
      (bind _returnvalue_2 (Class|FuncLibAbility|AddTargetstoEffectContainerSpec _returnvalue (Utilities|Array|MakeArray (Collision|MakeHitResult false false 0.0 0.0 (Transformation|GetActorLocation (LocalVariables|Get_Target)) (Transformation|GetActorLocation (LocalVariables|Get_Target)) "0,0,1" "0,0,1" 0 (LocalVariables|Get_Target)))))
      (Class|FuncLibAbility|ApplyEffectContainerSpec _returnvalue_2))))