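; Base skill projectile that flies along its forward vector at the speed set in Params and expires after the configured duration.
; With target tracking on, Tick points its velocity straight at the valid target every frame, with no gradual steering.
; Sphere overlaps are handled only with authority, applying an effect once per actor via the HitActors list.
; The projectile destroys itself after a hit when bDoOnce is set.
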(event OnComponentBeginOverlap(Sphere)
  (params (OverlappedComponent :type Primitive%20Component%20Object%20Reference) (OtherActor :type Actor%20Object%20Reference) (OtherComp :type Primitive%20Component%20Object%20Reference) (OtherBodyIndex :type Integer) (bFromSweep :type Boolean) (SweepResult :type Hit%20Result%20Structure%20%28by%20ref%29))
  (Variables|Default|SetOther%20Actor OtherActor)
  (Networking|SwitchHasAuthority
    (:Authority
      (Utilities|IsValid (Variables|Default|GetOther%20Actor)
        (:Is%20Valid
          (if (not (Utilities|Array|ContainsItem (Variables|Default|GetHitActors) (Variables|Default|GetOther%20Actor)))
            (Utilities|Array|AddUnique (Variables|Default|GetHitActors) (Variables|Default|GetOther%20Actor))
            (CallFunction|MakeandApplyEffect (Variables|Default|GetOther%20Actor))
            (if (.bdoonce (Variables|Default|GetParams))
              (Actor|DestroyActor))))))))

(event EventBeginPlay
  (bind _params (Variables|Default|GetParams))
  (Variables|/Script/Engine.MovementComponent|SetVelocity (Variables|Default|GetProjectileMovement) (* (Transformation|GetActorForwardVector) (.speed _params)))
  (Actor|SetLifeSpan (.duration _params)))

(event EventTick
  (params (DeltaSeconds :type Float%20%28single-precision%29))
  (bind _params (Variables|Default|GetParams))
  (if (and (.btracktarget _params) (Utilities|IsValid (.target _params)))
    (Variables|/Script/Engine.MovementComponent|SetVelocity (Variables|Default|GetProjectileMovement) (* (Math|Rotator|GetRotationXVector (Math|Rotator|FindLookatRotation (Transformation|GetActorLocation) (Transformation|GetActorLocation (.target _params)))) (.speed _params)))))

(fn ConstructionScript
  (|CallParentFunction))