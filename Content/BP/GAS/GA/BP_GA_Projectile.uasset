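; Gameplay Ability that fires a projectile-style skill actor from a montage.
; On successful activation it plays the montage, listens for Event.Montage tags and stops the avatar character's movement.
; A received tag found in the effect container map spawns the skill actor at a socket, using the avatar's rotation, with that container, event data and ability level.
; The ability ends when the montage completes, blends out, is interrupted or cancelled, or when activation fails.
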(event Ability|EventActivateAbility
  (|CallParentFunction) ; 此节点被禁用，将不会被调用。\n从引脚连出引线来编译功能。
)

(event Ability|EventOnEndAbility
  (params (bWasCancelled :type Boolean))
  (|CallParentFunction bWasCancelled) ; 此节点被禁用，将不会被调用。\n从引脚连出引线来编译功能。
)

(event EventOnActivateAbilitySuccess
  (bind (_asynctaskproxy _eventtag _eventdata) (|PlayMontageandWaitEventProxy "None" (Variables|Default|GetIn%20Montage%20to%20Play) "(GameplayTags=((TagName=\"Event.Montage\")))" 1.0 "None" true 1.0)
    (:then
      (bind _as角色 (Utilities|Casting|CastToCharacter (Ability|GetAvatarActorfromActorInfo)))
      (Components|Movement|StopMovementImmediately (Variables|/Script/Engine.Character|GetCharacterMovement _as角色)))
    (:OnMontageCompletedDelegate
      (Ability|EndAbility :!label _label))
    (:OnMontageBlendOutDelegate
      (goto _label))
    (:OnMontageInterruptedDelegate
      (goto _label))
    (:OnMontageCancelledDelegate
      (goto _label))
    (:OnEventReceivedDelegate
      (if (.ReturnValue (Utilities|Map|Find (Variables|Default|GetMap_GameplayEffectContainer) _eventtag))
        (Class|SRRoleBehavior|TrySpawnSkillActor(Message) (Ability|GetAvatarActorfromActorInfo) (Variables|Default|GetSkill%20Class) (.Value (Utilities|Map|Find (Variables|Default|GetMap_GameplayEffectContainer) _eventtag)) _eventdata (Ability|GetAbilityLevel) (Math|Transform|MakeTransform (Transformation|GetSocketLocation (Class|GameplayAbility|GetOwningComponentfromActorInfo) (Variables|Default|GetSpawn%20Socket%20Name)) (Transformation|GetActorRotation (Ability|GetAvatarActorfromActorInfo)) "1,1,1"))))))

(event EventOnActivateAbilityFailed
  (Ability|EndAbility))