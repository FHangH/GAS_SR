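; Test Gameplay Ability that plays a slowed jump-start montage and applies a test effect to its owner.
; On activation it commits the cooldown, ending immediately on failure, then waits on the montage and applies BP_GE_TEST when a TEST event arrives.
; Any montage finish or interruption ends the ability, with debug prints for start, end and cancel.
; Effect container and SetByCaller damage spec variants are left unconnected.
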(event Ability|EventOnEndAbility
  (params (bWasCancelled :type Boolean))
  (if bWasCancelled
    (Development|PrintString "GA TEST 1 Cancelled" true true "(R=1.000000,G=0.000000,B=0.000000,A=1.000000)" 1e+01)
    (else
      (Development|PrintString "GA TEST 1 End" true true "(R=0.000000,G=0.660000,B=1.000000,A=1.000000)" 1e+01))))

(event Ability|EventActivateAbility
  (bind _returnvalue (Ability|CommitAbilityCooldown false))
  (if _returnvalue
    (Development|PrintString "GA TEST 1" true true "(R=0.000000,G=0.660000,B=1.000000,A=1.000000)" 1e+01)
    (|PlayMontageandWaitEventProxy "None" "/Game/Assets/Mannequin/Animations/Montage/Montage_ThirdPersonJump_Start.Montage_ThirdPersonJump_Start" "(GameplayTags=((TagName=\"TEST\")))" 0.3 "None" true 1.0
      (:OnMontageCompletedDelegate
        (Ability|EndAbility :!label _label))
      (:OnMontageBlendOutDelegate
        (goto _label))
      (:OnMontageInterruptedDelegate
        (goto _label))
      (:OnMontageCancelledDelegate
        (goto _label))
      (:OnEventReceivedDelegate
        (Ability|ApplyGameplayEffectToOwner "/Game/TEST/BP_GE_TEST.BP_GE_TEST_C")))
    (else
      (Ability|EndAbility))))