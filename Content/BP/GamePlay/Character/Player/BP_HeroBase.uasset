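; BP_HeroBase is a player hero character Blueprint that handles basic movement and debug testing of Gameplay Ability System calls.
; Axis inputs move it along fixed world X and Y directions, and the Jump action makes it jump.
; Debug keys add, remove, query and level a test ability through the AbilitySystemComponent, printing feedback, while a numpad key sends a test gameplay event to itself.
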(event Input|ActionEvents|InputActionJump
  (params (Key :type Key%20Structure :default "None"))
  (:Pressed
    (Character|Jump)))

(event Input|AxisEvents|InputAxisMoveForward
  (params (AxisValue :type Float%20%28single-precision%29))
  (Pawn|Input|AddMovementInput "1.000000, 0, 0" AxisValue false))

(event Input|AxisEvents|InputAxisMoveRight
  (params (AxisValue :type Float%20%28single-precision%29))
  (Pawn|Input|AddMovementInput "0,1.000000, 0" AxisValue false))

(event Input|KeyboardEvents|Up
  (params (Key :type Key%20Structure :default "None"))
  (:Pressed
    (Class|SRAbilitySystemComponent|UpgradeAbilitybyClass (Variables|Default|GetAbilitySystemComponent) "/Game/BP/GAS/BP_GA_TEST_1.BP_GA_TEST_1_C" 1)
    (Development|PrintString "Upgarde Ability Level" true true "(R=0.095768,G=1.000000,B=0.000000,A=1.000000)")
    (Development|PrintString (Utilities|String|ToString(Integer) (Class|SRAbilitySystemComponent|GetAbilityLevelbyClass (Variables|Default|GetAbilitySystemComponent) "/Game/BP/GAS/BP_GA_TEST_1.BP_GA_TEST_1_C")) true true "(R=0.095768,G=1.000000,B=0.000000,A=1.000000)")))

(event Input|KeyboardEvents|Add
  (params (Key :type Key%20Structure :default "None"))
  (:Pressed
    (Class|SRAbilitySystemComponent|ServerAddNewAbility (Variables|Default|GetAbilitySystemComponent) "/Game/BP/GAS/BP_GA_TEST_1.BP_GA_TEST_1_C" 1)
    (Development|PrintString "Add New Ability - Jump" true true "(R=0.095768,G=1.000000,B=0.000000,A=1.000000)")))

(event Input|KeyboardEvents|Subtract
  (params (Key :type Key%20Structure :default "None"))
  (:Pressed
    (Class|SRAbilitySystemComponent|ServerRemoveAbilitybyClass (Variables|Default|GetAbilitySystemComponent) "/Game/BP/GAS/BP_GA_TEST_1.BP_GA_TEST_1_C")
    (Development|PrintString "Remove Ability - Jump" true true "(R=1.000000,G=0.980857,B=0.000000,A=1.000000)")))

(event Input|KeyboardEvents|Multiply
  (params (Key :type Key%20Structure :default "None"))
  (:Pressed
    (Development|PrintString (Utilities|String|ToString(Integer) (Class|SRAbilitySystemComponent|GetAbilityLevelbyClass (Variables|Default|GetAbilitySystemComponent) "/Game/BP/GAS/BP_GA_TEST_1.BP_GA_TEST_1_C")) true true "(R=0.095768,G=1.000000,B=0.000000,A=1.000000)")))

(event Input|KeyboardEvents|Down
  (params (Key :type Key%20Structure :default "None"))
  (:Pressed
    (Class|SRAbilitySystemComponent|UpgradeAbilitybyName (Variables|Default|GetAbilitySystemComponent) "GA1" -1)
    (Development|PrintString "Down Ability Level" true true "(R=1.000000,G=0.948679,B=0.000000,A=1.000000)")
    (Development|PrintString (Utilities|String|ToString(Integer) (Class|SRAbilitySystemComponent|GetAbilityLevelbyClass (Variables|Default|GetAbilitySystemComponent) "/Game/BP/GAS/BP_GA_TEST_1.BP_GA_TEST_1_C")) true true "(R=0.095768,G=1.000000,B=0.000000,A=1.000000)")))

(event Input|KeyboardEvents|NumPadZero
  (params (Key :type Key%20Structure :default "None"))
  (bind _self self)
  (:Pressed
    (Ability|SendGameplayEventtoActor _self "(TagName=\"TEST.State.1\")" (Utilities|Struct|MakeGameplayEventData "(TagName=\"\")" _self 0 0 0 "()" "(GameplayTags=)" "(GameplayTags=)" 123.0))))

(fn ConstructionScript)