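; Blueprint function library that converts between damage data and Gameplay Ability System cue parameters and tags.
; It builds gameplay cue parameters from a damage struct, carrying mitigated and raw magnitudes, hit location and normal, and the source ability system component.
; Damage type (physics, fire, ice) and status (normal, crit, real damage) become source tags.
; Two helper functions decode those tags back into enums, with fallback defaults.
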(fn MakeGameplayCueParamfromDamage
  (params (SourceASC :type Ability%20System%20Component%20Object%20Reference%20%28by%20ref%29) (DamageParam :type SR%20Damage%20Parameter%20Structure%20%28by%20ref%29))
  (bind (_hitresult _unmitigateddamage _mitigateddamage _type _status) (Utilities|Struct|BreakSRDamageParameter DamageParam))
  (Utilities|IsValid SourceASC
    (:Is%20Valid
      (LocalVariables|SetSourceASComponent SourceASC)
      (LocalVariables|SetHitResult _hitresult)
      (LocalVariables|SetRaw _unmitigateddamage)
      (LocalVariables|SetNormalized _mitigateddamage)
      (LocalVariables|SetAttackType _type)
      (LocalVariables|SetAttackStatus _status)
      (switch Utilities|FlowControl|Switch|SwitchonESRDamageType (LocalVariables|GetAttackType)
        (:Physics
          (LocalVariables|SetSourceTags "(GameplayTags=((TagName=\"Effect.Damage.Type.Physics\")))"))
        (:Fire
          (LocalVariables|SetSourceTags "(GameplayTags=((TagName=\"Effect.Damage.Type.Fire\")))"))
        (:Ice
          (LocalVariables|SetSourceTags "(GameplayTags=((TagName=\"Effect.Damage.Type.Ice\")))")))
      (switch Utilities|FlowControl|Switch|SwitchonESRDamageStatus (LocalVariables|GetAttackStatus)
        (:Normal
          (GameplayTags|AddGameplayTag (LocalVariables|GetSourceTags) "(TagName=\"Effect.Damage.Status.Normal\")" :!class /Script/GameplayTags.BlueprintGameplayTagLibrary))
        (:Crit
          (GameplayTags|AddGameplayTag (LocalVariables|GetSourceTags) "(TagName=\"Effect.Damage.Status.Crit\")" :!class /Script/GameplayTags.BlueprintGameplayTagLibrary))
        (:Realdamage
          (GameplayTags|AddGameplayTag (LocalVariables|GetSourceTags) "(TagName=\"Effect.Damage.Status.RealDamage\")" :!class /Script/GameplayTags.BlueprintGameplayTagLibrary)))
      (return (Ability|GameplayCue|MakeGameplayCueParameters :NormalizedMagnitude (LocalVariables|GetNormalized) :RawMagnitude (LocalVariables|GetRaw) :AggregatedSourceTags (LocalVariables|GetSourceTags) :Location (.impactpoint (LocalVariables|GetHitResult)) :Normal (.impactnormal (LocalVariables|GetHitResult)) :SourceObject (LocalVariables|GetSourceASComponent))))))

(fn GetDamageTypefromTagContainer
  (params (TagContainer :type Gameplay%20Tag%20Container%20Structure))
  (|SwitchGameplayTagContainer TagContainer
    (:Default
      (return "None"))
    (:%28GameplayTags=%28%28TagName="Effect.Damage.Type.Physics"%29%29%29
      (return "Physics"))
    (:%28GameplayTags=%28%28TagName="Effect.Damage.Type.Fire"%29%29%29
      (return "Fire"))
    (:%28GameplayTags=%28%28TagName="Effect.Damage.Type.Ice"%29%29%29
      (return "Ice"))))

(fn GetDamageStatusfromTagContainer
  (params (TagContainer :type Gameplay%20Tag%20Container%20Structure))
  (|SwitchGameplayTagContainer TagContainer
    (:Default
      (return "Normal"))
    (:%28GameplayTags=%28%28TagName="Effect.Damage.Status.Normal"%29%29%29
      (return "Normal"))
    (:%28GameplayTags=%28%28TagName="Effect.Damage.Status.Crit"%29%29%29
      (return "Crit"))
    (:%28GameplayTags=%28%28TagName="Effect.Damage.Status.RealDamage"%29%29%29
      (return "Realdamage"))))